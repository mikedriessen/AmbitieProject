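; Checkpoint actor that records itself and its number on the player character as the last checkpoint when the player overlaps its collision.
; The overlap also plays a sound at the player's effects volume and optionally switches the music.
; A separate event, not called here, optionally streams one named level in and another out without blocking, checking load state first.
; A save-game call is left disconnected for a later version.
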(event OnComponentBeginOverlap(Collision)
  (params (OverlappedComponent :type Primitive%20Component%20Object%20Reference) (OtherActor :type Actor%20Object%20Reference) (OtherComp :type Primitive%20Component%20Object%20Reference) (OtherBodyIndex :type Integer) (bFromSweep :type Boolean) (SweepResult :type Hit%20Result%20Structure%20%28by%20ref%29))
  (bind _asplayer_character (Utilities|Casting|CastToPlayerCharacter OtherActor))
  (Variables|/Game/GAME/Characters/PlayerCharacter.PlayerCharacter_C|SetLastCheckPoint _asplayer_character self)
  (Variables|/Game/GAME/Characters/PlayerCharacter.PlayerCharacter_C|SetCheckpointNumber _asplayer_character (Variables|Setup|GetCheckpointNumber))
  (Audio|PlaySound2D (Variables|Setup|GetSound) (Variables|/Game/GAME/Characters/PlayerCharacter.PlayerCharacter_C|GetEffectsMultiplier _asplayer_character) 1.0 0.0 0 0)
  (if (Variables|Music|GetPlayMusic?)
    (Default|FnSetMusic _asplayer_character (Variables|Music|GetSoundtrack) (Variables|Music|GetMusicID))))

(event Custom|EventLoadStreamingLevel
  (bind _loadlevelname (Variables|LoadLevel|GetLoadLevelName))
  (bind _unloadlevelname (Variables|LoadLevel|GetUnloadLevelName))
  (if (Variables|LoadLevel|GetLoadLevel?)
    (Utilities|FlowControl|Sequence
      (:then_0
        (if (not (Utilities|Name|Equal(Name) _loadlevelname "None"))
          (if (not (Class|LevelStreaming|IsLevelLoaded (Class|GameplayStatics|GetStreamingLevel _loadlevelname)))
            (Game|LoadStreamLevel(byName) _loadlevelname true))))
      (:then_1
        (if (not (Utilities|Name|Equal(Name) _unloadlevelname "None"))
          (if (Class|LevelStreaming|IsLevelLoaded (Class|GameplayStatics|GetStreamingLevel _unloadlevelname))
            (Game|UnloadStreamLevel(byName) _unloadlevelname false)))))))

(fn ConstructionScript)